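; EnemyBurningTest is a test enemy actor that plays a burn effect on itself, then may drop a health pickup.
; BeginPlay creates a dynamic material instance on the EnemyAnimationtest component and calls EnemyKilled after a short delay, without needing a hit.
; A timeline drives the material's Amount parameter.
; Its Update pin also leads through a Delay to DestroyActor, then a random chance to spawn HealthPickup at the actor's transform.
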(event `Enemy Killed`
  ;[1 1 1] When the enemy is hit, create a timeline to gradually adjust the "Amount" parameter
  (bind (_direction _newtrack_0) (`Timeline|Timeline_0`)
    (:`Update`
      (`MaterialInstanceDynamic.SetScalarParameterValue` (`self.Material 1`) "Amount" _newtrack_0)
      (`KismetSystemLibrary.Delay` 2.0)
      (`self.K2_DestroyActor`)
      (if (`KismetMathLibrary.RandomBool`)
        (`|SpawnActorFromClass` "/Game/Blueprints/Objects/HealthPickup.HealthPickup_C" (`self.GetTransform`) "Undefined" "OverrideRootScale" null null)))))

(event `self.ReceiveBeginPlay`
  ;[1 1 1] Creating a Material instance so variables can be changed and fire effect played
  (bind _returnvalue (`PrimitiveComponent.CreateDynamicMaterialInstance` (`self.EnemyAnimationtest`) 0 null "None"))
  (set `self.Material 1` _returnvalue)
  (`KismetSystemLibrary.Delay` 4.0)
  (`self.Enemy Killed`))

(fn `UserConstructionScript`)