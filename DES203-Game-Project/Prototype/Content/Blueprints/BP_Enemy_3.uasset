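; Enemy actor that fires a projectile on seeing a pawn and can burn away, randomly dropping a health pickup.
; A recursive Delay loop flipbooks idle or shooting texture arrays on the Cone's dynamic material, chosen by the Shooting flag set on sighting.
; EnemyKilled drives the material's Amount parameter by Timeline, then destroys the actor.
; The fire-breath overlap check that calls EnemyKilled is unwired, so never runs.
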(event `AwesomeLoop`
  (params (Array :type "Array of Texture Object Reference"))
  (bind _custom_index (`self.Custom Index`))
  ;[0.7934 0.02617 0.02617] Hedda's (Awesome) Animation Loop
  ;;[0.7934 0.02617 0.02617] Total Length of Animation is Based on Amount of Frames in the Array
  (bind _output_get (set `self.Amount of Frames` (`KismetArrayLibrary.Array_Length` Array)))
  (set `self.Total Animation Length` (* _output_get 0.2))
  ;;[0.7934 0.02617 0.02617] Where we are in the Array
  (bind _result (`/Engine/EditorBlueprintResources/StandardMacros.IncrementInt` _custom_index)
    (:`  `
      ;;[0.7934 0.02617 0.02617] Amount of Frames - 1 = last index of the Array
      (bind _result_2 (`/Engine/EditorBlueprintResources/StandardMacros.DecrementInt` (`self.Amount of Frames`))
        (:`  `
          (if (< _result _result_2)
            (`self.Set Texture` (`|GetArrayItem` Array _custom_index))
            ;;[0.7934 0.02617 0.02617] Length Per Frame
            (`KismetSystemLibrary.Delay` (/ (`self.Total Animation Length`) (`self.Amount of Frames`)))
            ;;[0.7934 0.02617 0.02617] Loop Continues Here
            (`self.AwesomeLoop` Array)
            (else
              ;;[0.7934 0.02617 0.02617] Loop Ends Here
              (set `self.Custom Index` -1))))))))

(event `Set Texture`
  (params (Frame :type "Texture Object Reference"))
  (`MaterialInstanceDynamic.SetTextureParameterValue` (`self.Material 1`) "ObjectTexture" Frame))

(event `PlayIdleAnimation`
  ;[1 1 1] Idle Animatino
  (`self.AwesomeLoop` (`self.Idle`))
  (`KismetSystemLibrary.Delay` (`self.Total Animation Length`))
  (`self.CheckAnimation`))

(event `CheckAnimation`
  (if (`self.Shooting`)
    (`self.PlayShootingAnimation`)
    (else
      (`self.PlayIdleAnimation`))))

(event `PlayShootingAnimation`
  ;[1 1 1] Play Shooting animatin
  (`self.AwesomeLoop` (`self.ShootingAnimation`))
  (`KismetSystemLibrary.Delay` (`self.Total Animation Length`))
  (`self.CheckAnimation`))

(event `Enemy Killed`
  ;[1 1 1] When the enemy is hit, create a timeline to gradually adjust the "Amount" parameter
  (bind (_direction _newtrack_0) (`Timeline|Timeline_0`)
    (:`Update`
      (`MaterialInstanceDynamic.SetScalarParameterValue` (`self.Material 1`) "Amount" _newtrack_0)
      (`KismetSystemLibrary.Delay` 2.0)
      (`self.K2_DestroyActor`)
      (if (`KismetMathLibrary.RandomBool`)
        (`|SpawnActorFromClass` "/Game/Blueprints/Objects/HealthPickup.HealthPickup_C" (`self.GetTransform`) "Undefined" "OverrideRootScale" null null)))))

(event `self.ReceiveBeginPlay`
  ;[1 1 1] Creating a Material instance so variables can be changed and fire effect played
  (bind _returnvalue (`PrimitiveComponent.CreateDynamicMaterialInstance` (`self.Cone`) 0 null "None"))
  (set `self.Material 1` _returnvalue))

(event `self.PawnSensing.OnSeePawn`
  (params (Pawn :type "Pawn Object Reference"))
  ;[1 1 1] Spawn the Projecitle
  (set `self.Shooting` true)
  (`KismetSystemLibrary.Delay` 0.7)
  (`|SpawnActorFromClass` "/Game/Blueprints/BP_EnemyProjectile.BP_EnemyProjectile_C" (`self.GetTransform`) "AdjustIfPossibleButDontSpawnIfColliding" "OverrideRootScale" null null)
  (set `self.Shooting` false))

(fn `UserConstructionScript`)