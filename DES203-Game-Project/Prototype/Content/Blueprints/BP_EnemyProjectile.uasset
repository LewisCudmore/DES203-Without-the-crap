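; Enemy projectile that lobs itself in an arc toward where the player is predicted to be and damages them on contact.
; BeginPlay leads the target by velocity times distance over ProjectileSpeed, then feeds SuggestProjectileVelocityCustomArc's result into ProjectileMovement.
; Sphere overlap with BP_ThirdPersonCharacter sets its Damage and calls DamagePlayer, without destroying the projectile.
; The construction script sets a short lifespan; an earlier arc attempt remains unconnected.
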(event `self.ReceiveBeginPlay`
  (bind _returnvalue (`GameplayStatics.GetPlayerCharacter` 0))
  ;[1 1 1] Calculating the Arch needed
  (bind _outlaunchvelocity (`GameplayStatics.SuggestProjectileVelocity_CustomArc` (`self.K2_GetActorLocation`) (+ (`self.K2_GetActorLocation` _returnvalue) (* (`self.GetVelocity` _returnvalue) (/ (`self.GetDistanceTo` _returnvalue) (`self.ProjectileSpeed`))))))
  (set `MovementComponent.Velocity` _outlaunchvelocity (`self.ProjectileMovement`)))

(event `self.Sphere.OnComponentBeginOverlap`
  (params (OverlappedComponent :type "PrimitiveComponent Object Reference") (OtherActor :type "Actor Object Reference") (OtherComp :type "PrimitiveComponent Object Reference") (OtherBodyIndex :type Integer) (bFromSweep :type Boolean) (SweepResult :type "HitResult Structure (by ref)"))
  ;[1 1 1] When Hitting the player deal damage
  (bind _asbp_third_person_character (cast `/Game/ThirdPerson/Blueprints/CameraAndCharacter/BP_ThirdPersonCharacter` OtherActor))
  (set `/Game/ThirdPerson/Blueprints/CameraAndCharacter/BP_ThirdPersonCharacter.Damage` 1 _asbp_third_person_character)
  (`/Game/ThirdPerson/Blueprints/CameraAndCharacter/BP_ThirdPersonCharacter.DamagePlayer` _asbp_third_person_character))

(fn `UserConstructionScript`
  (`self.SetLifeSpan` 2.0))