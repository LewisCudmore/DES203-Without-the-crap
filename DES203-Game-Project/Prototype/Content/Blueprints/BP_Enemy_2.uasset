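; Enemy that approaches the player on sight via pawn sensing and AI MoveTo, then detonates after a delay.
; Detonation damages the player if inside the Explosion overlap and destroys the enemy either way.
; Texture arrays drive idle, charging and detonating flipbook animations through a dynamic material, selected by state flags.
; EnemyKilled animates the material's Amount for a burn death, but its fire-breath overlap trigger is disconnected.
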(event `Set Texture`
  (params (Frame :type "Texture Object Reference"))
  (`MaterialInstanceDynamic.SetTextureParameterValue` (`self.Material1`) "ObjectTexture" Frame))

(event `PlayIdleAnimation`
  ;[1 1 1] Idle Animatino
  (for _array_element (`self.Idle`)
    (`self.Set Texture` _array_element)
    (`KismetSystemLibrary.Delay` 1.0)
    (`KismetSystemLibrary.PrintString` (`KismetSystemLibrary.GetDisplayName` _array_element)))
  (`KismetSystemLibrary.Delay` 0.2)
  (`self.CheckAnimation`))

(event `PlayDetonatingAnimation`
  ;[1 1 1] Detonating Animation
  (for _array_element (`self.DetonatingAnimation`)
    (`MaterialInstanceDynamic.SetTextureParameterValue` (`self.Material1`) "ObjectTexture" _array_element)
    (`KismetSystemLibrary.PrintString` "Detonating")))

(event `CheckAnimation`
  ;[1 1 1] Check what animation should be playing
  (if (`self.EnemyCharging`)
    (`self.PlayChargingAnimation`)
    (elif (`self.Detonating`)
      (`self.PlayDetonatingAnimation`)
      (else
        (`self.PlayIdleAnimation`)))))

(event `PlayChargingAnimation`
  ;[1 1 1] Swapping the base map for the running effect
  (for _array_element (`self.Charging`)
    (`MaterialInstanceDynamic.SetTextureParameterValue` (`self.Material1`) "ObjectTexture" _array_element)))

(event `EnemyKilled`
  ;[1 1 1] When the enemy is hit, create a timeline to gradually adjust the "Amount" parameter
  (bind (_direction _newtrack_0) (`Timeline|Timeline_0`)
    (:`Update`
      (`MaterialInstanceDynamic.SetScalarParameterValue` (`self.Material1`) "Amount" _newtrack_0)
      (`KismetSystemLibrary.Delay` 2.0)
      (`self.K2_DestroyActor`))))

(event `self.ReceiveBeginPlay`
  ;[1 1 1] Creating a Material instance so variables can be changed and fire effect played
  (bind _returnvalue (`PrimitiveComponent.CreateDynamicMaterialInstance` (`self.Cube`) 0 null "None"))
  (set `self.Material1` _returnvalue)
  (`self.CheckAnimation`))

(event `self.PawnSensing.OnSeePawn`
  (params (Pawn :type "Pawn Object Reference"))
  ;[1 1 1] If Enemy is seeing the player then move towards the player
  (set `self.PlayerSeen` true)
  (if (not (`self.Detonating`))
    (`self.ApproachPlayer`)))

(event `CheckPlayerClose`
  ;[1 1 1] Checking if the player is close enough to be damaged
  (bind _returnvalue (`GameplayStatics.GetActorOfClass` "/Game/ThirdPerson/Blueprints/CameraAndCharacter/BP_ThirdPersonCharacter.BP_ThirdPersonCharacter_C"))
  (if (`PrimitiveComponent.IsOverlappingActor` (`self.Explosion`) _returnvalue)
    (set `self.CloseEnough` true)
    (else
      (set `self.CloseEnough` false))))

(event `ApproachPlayer`
  ;[1 1 1] If Enemy is seeing the player then move towards the player
  (if (`self.PlayerSeen`)
    (`|AIMoveTo` self (0.0 0.0 0.0) (`GameplayStatics.GetPlayerCharacter` 0)
      (:`then`
        (set `self.EnemyCharging` true))
      (:`OnSuccess`
        (set `self.EnemyCharging` false)
        (`self.Detonate!`)))))

(event `Detonate!`
  ;[1 1 1] Detonating the Enemy
  (set `self.Detonating` true)
  (`KismetSystemLibrary.Delay` 2.0)
  (`self.CheckPlayerClose`)
  (if (`self.CloseEnough`)
    (`self.K2_DestroyActor`)
    (bind _returnvalue (`GameplayStatics.GetActorOfClass` "/Game/ThirdPerson/Blueprints/CameraAndCharacter/BP_ThirdPersonCharacter.BP_ThirdPersonCharacter_C"))
    (set `/Game/ThirdPerson/Blueprints/CameraAndCharacter/BP_ThirdPersonCharacter.Damage` 2 _returnvalue)
    (`/Game/ThirdPerson/Blueprints/CameraAndCharacter/BP_ThirdPersonCharacter.DamagePlayer` _returnvalue)
    (else
      (`self.K2_DestroyActor`))))

(fn `FollowPlayer`)

(fn `UserConstructionScript`)