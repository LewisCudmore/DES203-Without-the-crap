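; BP_Enemy_1 is an enemy character that walks back and forth along world X and can burn away when killed.
; Tick drives movement, flipping SwapDirection through three-second Delays.
; EnemyKilled plays a timeline on the Sphere's dynamic material "Amount" parameter for the fire effect, destroying the actor after a delay.
; The overlap check for a fire-breathing player that calls EnemyKilled is disconnected, so it never runs.
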(event `EnemyKilled`
  ;[1 1 1] When the enemy is hit, create a timeline to gradually adjust the "Amount" parameter
  (bind (_direction _newtrack_0) (`Timeline|BurningEnemy`)
    (:`Update`
      (`MaterialInstanceDynamic.SetScalarParameterValue` (`self.Material1`) "Amount" _newtrack_0)
      (`KismetSystemLibrary.Delay` 2.0)
      (`self.K2_DestroyActor`))))

(event `self.ReceiveBeginPlay`
  ;[1 1 1] Creating a Material instance so variables can be changed and fire effect played
  (bind _returnvalue (`PrimitiveComponent.CreateDynamicMaterialInstance` (`self.Sphere`) 0 null "None"))
  (set `self.Material1` _returnvalue))

(event `self.ReceiveTick`
  (params (DeltaSeconds :type "Float (single-precision)"))
  ;[1 1 1] Enemy walking back and forth
  (if (`self.SwapDirection`)
    (`self.AddMovementInput` (-1.0 0.0 0.0))
    (`KismetSystemLibrary.Delay` 3.0)
    (set `self.SwapDirection` false)
    (else
      (`self.AddMovementInput` (1.0 0.0 0.0))
      (`KismetSystemLibrary.Delay` 3.0)
      (set `self.SwapDirection` true))))

(fn `UserConstructionScript`)