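; WaterClass is a water volume actor that plays a flowing-water sound at its location on BeginPlay.
; Its collision box flags BP_ThirdPersonCharacter as in water on begin overlap and clears that flag on end overlap.
; Entering also calls WaterDamage, which sets the character's Damp flag while it overlaps the box.
; An unwired branch that would raise Dryness and destroy the player at its limit never runs.
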(event `self.ReceiveBeginPlay`
  (`GameplayStatics.PlaySoundAtLocation` "/Game/Assets/CompleteAssets/Assets_Sound/SFX/SFX_Environment/flowing_water.flowing_water" (`self.K2_GetActorLocation`) (struct) 8.0 1.0 0.0 (`self.Attenuation Settings`) null null null))

(event `self.CollisionBox.OnComponentBeginOverlap`
  (params (OverlappedComponent :type "PrimitiveComponent Object Reference") (OtherActor :type "Actor Object Reference") (OtherComp :type "PrimitiveComponent Object Reference") (OtherBodyIndex :type Integer) (bFromSweep :type Boolean) (SweepResult :type "HitResult Structure (by ref)"))
  (bind _asbp_third_person_character (cast `/Game/ThirdPerson/Blueprints/CameraAndCharacter/BP_ThirdPersonCharacter` OtherActor))
  (set `/Game/ThirdPerson/Blueprints/CameraAndCharacter/BP_ThirdPersonCharacter.IsPlayerCharacterInWater` true _asbp_third_person_character)
  (`self.WaterDamage`))

(event `WaterDamage`
  ;[1 1 1] Updating Damp Value
  (bind _returnvalue (`GameplayStatics.GetActorOfClass` "/Game/ThirdPerson/Blueprints/CameraAndCharacter/BP_ThirdPersonCharacter.BP_ThirdPersonCharacter_C"))
  (if (`PrimitiveComponent.IsOverlappingActor` (`self.CollisionBox`) _returnvalue)
    (if (not (`/Game/ThirdPerson/Blueprints/CameraAndCharacter/BP_ThirdPersonCharacter.Damp` _returnvalue))
      (set `/Game/ThirdPerson/Blueprints/CameraAndCharacter/BP_ThirdPersonCharacter.Damp` true _returnvalue))))

(event `self.CollisionBox.OnComponentEndOverlap`
  (params (OverlappedComponent :type "PrimitiveComponent Object Reference") (OtherActor :type "Actor Object Reference") (OtherComp :type "PrimitiveComponent Object Reference") (OtherBodyIndex :type Integer))
  (bind _asbp_third_person_character (cast `/Game/ThirdPerson/Blueprints/CameraAndCharacter/BP_ThirdPersonCharacter` OtherActor))
  (set `/Game/ThirdPerson/Blueprints/CameraAndCharacter/BP_ThirdPersonCharacter.IsPlayerCharacterInWater` false _asbp_third_person_character))

(fn `UserConstructionScript`)