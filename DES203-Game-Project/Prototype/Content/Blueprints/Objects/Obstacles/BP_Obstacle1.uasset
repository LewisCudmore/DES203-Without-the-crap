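; BP_Obstacle1 is an obstacle actor that burns away and destroys itself when its EnemyKilled event fires.
; BeginPlay sets its damage value and creates a dynamic material instance on the Box.
; EnemyKilled plays a timeline that drives the material's Amount parameter for the burn effect, with a delayed destroy chained off the timeline update.
; The overlap check for a fire-breathing player is disconnected, so nothing here triggers EnemyKilled.
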(event `self.ReceiveBeginPlay`
  ;[0.5529 0.07059 0.03529] Prep Obstacle
  (set `self.DamageValue` 2)
  ;[1 1 1] Create Dynamic Material Instance for Burning
  (bind _returnvalue (`PrimitiveComponent.CreateDynamicMaterialInstance` (`self.Box`) 0 null "None"))
  (set `self.Material1` _returnvalue))

(event `self.ReceiveTick`
  (params (DeltaSeconds :type "Float (single-precision)"))
  ;[0.5529 0.5529 0.5529] Checking if the player is colliding with the Enemy
)

(event `EnemyKilled`
  ;[1 1 1] Burning Effect
  (bind (_direction _newtrack_0) (`Timeline|Timeline_0`)
    (:`Update`
      (`MaterialInstanceDynamic.SetScalarParameterValue` (`self.Material1`) "Amount" _newtrack_0)
      (`KismetSystemLibrary.Delay` 2.0)
      (`self.K2_DestroyActor`))))

(fn `UserConstructionScript`)