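; Collectible candy pickup that adds a point to the player's score when the third-person character overlaps it.
; On BeginPlay it applies a texture chosen by CandyNumber through a dynamic material instance and starts a timeline-driven yaw wiggle.
; Collection is guarded by a one-shot flag, then freezes the current wiggle yaw and plays a pitch spin timeline before destroying the actor.
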(event `self.ReceiveBeginPlay`
  ;[1 1 1] Set Colour of Collectable
  (bind _returnvalue (`PrimitiveComponent.CreateDynamicMaterialInstance` (`self.MergedCandy`) 0 "/Game/Assets/CompleteAssets/Assets_3D/Candy/CandyMaterial.CandyMaterial" "None"))
  (bind _output_get (set `self.MaterialInstance` _returnvalue))
  (`MaterialInstanceDynamic.SetTextureParameterValue` _output_get "BaseColor" (`|GetArrayItem` (`self.TextureArray`) (`self.CandyNumber`)))
  ;[1 0.05035 0.05035] Trigger Wiggle Animation
  (`self.Animation_CandyWiggle`))

(event `self.ReceiveActorBeginOverlap`
  (params (OtherActor :type "Actor Object Reference"))
  ;[0.07832 0.146 1] This checks to ensure it is the player that overlaps it, so nothing else can overlap the collectible and destroy it
  (if (`self.CandyCollected`)
    _
    (elif (== (`GameplayStatics.GetObjectClass` OtherActor) "/Game/ThirdPerson/Blueprints/CameraAndCharacter/BP_ThirdPersonCharacter.BP_ThirdPersonCharacter_C")
      (bind _asbp_third_person_character (cast `/Game/ThirdPerson/Blueprints/CameraAndCharacter/BP_ThirdPersonCharacter` (`GameplayStatics.GetPlayerCharacter` 0)))
      (set `self.CandyCollected` true)
      (set `/Game/ThirdPerson/Blueprints/CameraAndCharacter/BP_ThirdPersonCharacter.Points` (+ (`/Game/ThirdPerson/Blueprints/CameraAndCharacter/BP_ThirdPersonCharacter.Points` _asbp_third_person_character) 1.0) _asbp_third_person_character)
      ;[1 0.05035 0.05035] Candy Collected Spin
      (`self.Animation_CandySpin`))))

(event `Animation_CandyWiggle`
  ;[1 0.05035 0.05035] Candy Wiggle
  (bind (_direction _wiggle) (`Timeline|TL_WiggleValue` :!label _label)
    (:`Update`
      (`SceneComponent.K2_SetRelativeRotation` (`self.MergedCandy`) (`KismetMathLibrary.MakeRotator` 0.0 0.0 _wiggle) false false))))

(event `Animation_CandySpin`
  ;[1 0.05035 0.05035] Candy Spin
  (`|ExecutionSequence`
    (:`then_0`
      (set `self.SpinAngle_Z` (stale `Animation_CandyWiggle` _wiggle))
      (goto _label :!via `Stop`))
    (:`then_1`
      (bind (_direction _spin) (`Timeline|TL_SpinValue`)
        (:`Update`
          (`SceneComponent.K2_SetRelativeRotation` (`self.MergedCandy`) (`KismetMathLibrary.MakeRotator` 0.0 _spin (`self.SpinAngle_Z`)) false false))
        (:`Finished`
          ;[0 0 0] Candy is collected (dunno who made this tbf)
          (`self.K2_DestroyActor`)
          (`KismetSystemLibrary.PrintString` "Collectible Collected" true true (struct :`G` 0.063701 :`B` 1.0 :`A` 1.0)))))))

(fn `UserConstructionScript`)